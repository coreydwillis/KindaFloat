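; GroundDestroy is an actor that destroys itself after a five-step audio countdown, presumably removing the ground at level start.
; BeginPlay reads the level number from the GlobalVars game instance, adding an extra delay on level 3 before the one-second-spaced countdown clips.
; It then plays explosion and wind sounds around its destruction, and the Destroyed event spawns an explosion effect at the Cube's location.
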(event `self.ReceiveBeginPlay`
  (`KismetSystemLibrary.DelayUntilNextTick`)
  (bind _asglobal_vars (cast `/Game/Blueprints/GlobalVars` (`GameplayStatics.GetGameInstance`)))
  (if (== (`/Game/Blueprints/GlobalVars.CurrentLevelNumber` _asglobal_vars) 3)
    (`KismetSystemLibrary.Delay` 11.0))
  (`GameplayStatics.PlaySound2D` "/Game/Audio/Kinda_Float_5.Kinda_Float_5" 1.0 1.0 0.0 null null)
  (`KismetSystemLibrary.Delay` 1.0)
  (`GameplayStatics.PlaySound2D` "/Game/Audio/Kinda_Float_4.Kinda_Float_4" 1.0 1.0 0.0 null null)
  (`KismetSystemLibrary.Delay` 1.0)
  (`GameplayStatics.PlaySound2D` "/Game/Audio/Kinda_Float_3wav.Kinda_Float_3wav" 1.0 1.0 0.0 null null)
  (`KismetSystemLibrary.Delay` 1.0)
  (`GameplayStatics.PlaySound2D` "/Game/Audio/Kinda_Float_2wav.Kinda_Float_2wav" 1.0 1.0 0.0 null null)
  (`KismetSystemLibrary.Delay` 1.0)
  (`GameplayStatics.PlaySound2D` "/Game/Audio/Kinda_Float_1.Kinda_Float_1" 1.0 1.0 0.0 null null)
  (`KismetSystemLibrary.Delay` 1.0)
  (`GameplayStatics.PlaySound2D` "/Game/StarterContent/Audio/Explosion02.Explosion02" 2.0 0.85 0.0 null null)
  (`self.K2_DestroyActor`)
  (`GameplayStatics.PlaySound2D` "/Game/StarterContent/Audio/Starter_Wind05.Starter_Wind05" 0.65 1.0 0.0 null null))

(event `self.ReceiveDestroyed`
  (`|SpawnActorFromClass` "/Game/StarterContent/Blueprints/Blueprint_Effect_Explosion.Blueprint_Effect_Explosion_C" (`KismetMathLibrary.Conv_VectorToTransform` (`SceneComponent.K2_GetComponentLocation` (`self.Cube`))) "Undefined" "OverrideRootScale" null null))

(fn `UserConstructionScript`)
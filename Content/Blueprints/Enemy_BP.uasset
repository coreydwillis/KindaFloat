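; Enemy_BP is an enemy actor that fires Projectile_BP shots at a level-dependent rate.
; Tick reads CurrentLevelNumber from the GlobalVars game instance and sets EnemySpeed as the delay between shots, shorter from level four onward.
; A Delay inside Tick paces the repeated spawns at the SpawnProjectile component's transform.
; On destruction it issues a spawn at the Head component's location, with no class specified.
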(event `self.ReceiveTick`
  (params (DeltaSeconds :type "Float (single-precision)"))
  (bind _asglobal_vars (cast `/Game/Blueprints/GlobalVars` (`GameplayStatics.GetGameInstance`)))
  (if (>= (`/Game/Blueprints/GlobalVars.CurrentLevelNumber` _asglobal_vars) 4)
    (set `self.EnemySpeed` 0.5)
    (else
      (set `self.EnemySpeed` 1.5)))
  (`KismetSystemLibrary.Delay` (`self.EnemySpeed`))
  (`|SpawnActorFromClass` "/Game/Blueprints/Projectile_BP.Projectile_BP_C" (`SceneComponent.K2_GetComponentToWorld` (`self.spawn_projectile`)) "Undefined" "OverrideRootScale" null null))

(event `self.ReceiveDestroyed`
  (`|SpawnActorFromClass` "/Game/StarterContent/Blueprints/Blueprint_Effect_Explosion.Blueprint_Effect_Explosion_C" (`KismetMathLibrary.Conv_VectorToTransform` (`SceneComponent.K2_GetComponentLocation` (`self.Head`))) "Undefined" "OverrideRootScale" null null))

(fn `UserConstructionScript`)
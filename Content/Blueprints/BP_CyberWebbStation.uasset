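; BP_CyberWebbStation is the goal point that wins the game when the player brings enough fragments to it.
; On Box overlap, it compares the BP_FirstPersonCharacter's Fragments against FragmentsGoal, then either sets the win flags and calls GameOverEvent or plays a "more chips" sound.
; An IsPlaying flag with a delayed reset keeps that sound from retriggering on repeated overlaps.
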(event `self.Box.OnComponentBeginOverlap`
  (params (OverlappedComponent :type "PrimitiveComponent Object Reference") (OtherActor :type "Actor Object Reference") (OtherComp :type "PrimitiveComponent Object Reference") (OtherBodyIndex :type Integer) (bFromSweep :type Boolean) (SweepResult :type "HitResult Structure (by ref)"))
  (bind _asbp_first_person_character (cast `/Game/Blueprints/BP_FirstPersonCharacter` OtherActor))
  (if (>= (`/Game/Blueprints/BP_FirstPersonCharacter.Fragments` _asbp_first_person_character) (`/Game/Blueprints/BP_FirstPersonCharacter.FragmentsGoal` _asbp_first_person_character))
    (set `/Game/Blueprints/BP_FirstPersonCharacter.GameOver` true _asbp_first_person_character)
    (set `/Game/Blueprints/BP_FirstPersonCharacter.GameLost` false _asbp_first_person_character)
    (`/Game/Blueprints/BP_FirstPersonCharacter.GameOverEvent` _asbp_first_person_character)
    (elif (not (`self.IsPlaying?`))
      (set `self.IsPlaying?` true)
      (`GameplayStatics.PlaySound2D` "/Game/Audio/Kinda_Float_more_chips.Kinda_Float_more_chips" 3.0 1.0 0.0 null null)
      (`KismetSystemLibrary.Delay` 5.0)
      (set `self.IsPlaying?` false))))

(fn `UserConstructionScript`)